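; EnemyManagerBP is an enemy spawner that keeps adding EnemyBP actors to the level over time.
; Tick counts down a timer, then calls SpawnEnemy and resets the delay by interpolating from MinSpawnRate to MaxSpawnRate over game time, with random jitter.
; SpawnEnemy picks a randomized position around the world origin from SpawnRadius, retries recursively if spawning fails, and records successes in Enemies.
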(event EventBeginPlay
  (bind _minspawnrate (Variables|Default|GetminSpawnRate))
  (bind _returnvalue (Actor|GetActorOfClass "/Game/VRTemplate/Blueprints/VRGameMode.VRGameMode_C"))
  (Variables|Default|Setgm _returnvalue)
  (bind _returnvalue_2 (Actor|GetActorOfClass "/Game/VRTemplate/Blueprints/VRPawn.VRPawn_C"))
  (Variables|Default|Setplayer _returnvalue_2)
  (Variables|Default|SetspawnRate _minspawnrate)
  (Variables|Default|SetcurrSpawnRate _minspawnrate))

(event EventTick
  (params (DeltaSeconds :type Float%20%28single-precision%29))
  (bind _output_get (Variables|Default|SetspawnRate (- (Variables|Default|GetspawnRate) DeltaSeconds)))
  (if (<= _output_get 0.0)
    (CallFunction|SpawnEnemy)
    (CallFunction|UpdateSpawnRate)))

(fn ConstructionScript)

(fn SpawnEnemy
  (bind _returnvalue (Math|Random|RandomFloatinRange 0.0 3.6e+02))
  (bind _returnvalue_2 (Math|Random|RandomFloatinRange 0.7 1.3))
  (bind _spawnradius (Variables|Default|GetspawnRadius))
  (bind _returnvalue_3 (* _spawnradius _returnvalue_2))
  (bind _returnvalue_4 (Game|SpawnActorfromClass "/Game/Blueprints/EnemyBP.EnemyBP_C" (Math|Conversions|ToTransform(Vector) (Math|Vector|MakeVector (* _returnvalue_3 (Math|Trig|Cos(Degrees) _returnvalue)) (* _returnvalue_3 (Math|Trig|Sin(Degrees) _returnvalue)) 1e+02)) "AdjustIfPossibleButDontSpawnIfColliding" "MultiplyWithRoot" 0 0))
  (Utilities|IsValid _returnvalue_4
    (:Is%20Valid
      (Utilities|Array|Add (Variables|Default|Getenemies) _returnvalue_4))
    (:Is%20Not%20Valid
      (CallFunction|SpawnEnemy))))

(fn UpdateSpawnRate
  (Variables|Default|SetspawnRate (* (Math|Float|Lerp (Variables|Default|GetminSpawnRate) (Variables|Default|GetmaxSpawnRate) (Math|Float|Min(Float) (/ (Utilities|Time|GetGameTimeinSeconds) (Variables|Default|GetmaxSpawnTime)) 1.0)) (Math|Random|RandomFloatinRange 0.7 1.3))))