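; A VR sword that the player can grab and use to kill EnemyBP characters on contact.
; When its box collider overlaps an enemy and the VRPawn's SwordAllowAttack flag is set, it plays an impact sound and right-hand haptics, then calls Die on the enemy.
; Grab and drop events set IsHoldingSword on the pawn, and debug prints trace each collision outcome.
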(event OnGrabbed(GrabComponent)
  ;[0 0 0] Set Pawn Hold Sword
  (bind _returnvalue (Actor|GetActorOfClass "/Game/VRTemplate/Blueprints/VRPawn.VRPawn_C"))
  (Variables|/Game/VRTemplate/Blueprints/VRPawn.VRPawn_C|SetIsHoldingSword _returnvalue true))

(event OnDropped(GrabComponent)
  ;[0 0 0] Set Pawn Drop Sword
  (bind _returnvalue (Actor|GetActorOfClass "/Game/VRTemplate/Blueprints/VRPawn.VRPawn_C"))
  (Variables|/Game/VRTemplate/Blueprints/VRPawn.VRPawn_C|SetIsHoldingSword _returnvalue false))

(event OnComponentHit(BoxCollider)
  (params (HitComponent :type Primitive%20Component%20Object%20Reference) (OtherActor :type Actor%20Object%20Reference) (OtherComp :type Primitive%20Component%20Object%20Reference) (NormalImpulse :type Vector :default "0, 0, 0") (Hit :type Hit%20Result%20Structure%20%28by%20ref%29)))

(event OnComponentBeginOverlap(BoxCollider)
  (params (OverlappedComponent :type Primitive%20Component%20Object%20Reference) (OtherActor :type Actor%20Object%20Reference) (OtherComp :type Primitive%20Component%20Object%20Reference) (OtherBodyIndex :type Integer) (bFromSweep :type Boolean) (SweepResult :type Hit%20Result%20Structure%20%28by%20ref%29))
  ;[0 0 0] Collision with Ninja
  (Development|PrintString "Collision" true true "(R=0.237488,G=1.000000,B=0.320816,A=1.000000)")
  (bind _asenemy_bp (Utilities|Casting|CastToEnemyBP OtherActor)
    (:then
      (bind _returnvalue (Actor|GetActorOfClass "/Game/VRTemplate/Blueprints/VRPawn.VRPawn_C"))
      (if (Variables|/Game/VRTemplate/Blueprints/VRPawn.VRPawn_C|GetSwordAllowAttack _returnvalue)
        (Development|PrintString "Sword Allow Attack" true true "(R=0.947161,G=1.000000,B=0.031250,A=1.000000)")
        (Audio|PlaySoundatLocation "/Game/Assets/SoundEffects/sword-impact.sword-impact" (Transformation|GetActorLocation _asenemy_bp) "0, 0, 0" 1.0 1.0 0.0 0 0 0 0)
        (Class|PlayerController|PlayHapticEffect (Game|GetPlayerController 0) "/Game/VRTemplate/Haptics/PistolFireHapticEffect.PistolFireHapticEffect" "Right" 1.0 false)
        (Default|Die _asenemy_bp)
        (else
          (Development|PrintString "Sword Not Allow Attack" true true "(R=0.773007,G=0.135962,B=1.000000,A=1.000000)"))))
    (:CastFailed
      (Development|PrintString "Cast Failed" true true "(R=1.000000,G=0.000000,B=0.056551,A=1.000000)"))))

(event EventBeginPlay)

(event Collision|EventActorBeginOverlap
  (params (OtherActor :type Actor%20Object%20Reference)))

(event EventTick
  (params (DeltaSeconds :type Float%20%28single-precision%29)))

(fn ConstructionScript)